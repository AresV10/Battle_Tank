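; Player-controlled tank Blueprint with basic camera-rig rotation and stepped hull movement.
; The AxisX and AxisY inputs yaw the XYgimble and pitch the SpringArm separately, using raw axis values with no clamping or delta-time scaling.
; Forward and Back presses shift TankHull by a fixed swept local offset, so it moves once per press rather than continuously.
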(event `InputAxis|AxisX`
  (params (AxisValue :type "Float (single-precision)"))
  (`SceneComponent.K2_AddLocalRotation` (`self.XYgimble`) (`KismetMathLibrary.MakeRotator` 0.0 0.0 AxisValue) false false))

(event `InputAxis|AxisY`
  (params (AxisValue :type "Float (single-precision)"))
  (`SceneComponent.K2_AddLocalRotation` (`self.SpringArm`) (`KismetMathLibrary.MakeRotator` 0.0 AxisValue) false false))

(event `InputAction|Forward`
  (params (Key :type "Key Structure"))
  (:`Pressed`
    (`SceneComponent.K2_AddLocalOffset` (`self.TankHull`) (50.0 0.0 0.0) true false)))

(event `InputAction|Back`
  (params (Key :type "Key Structure"))
  (:`Pressed`
    (`SceneComponent.K2_AddLocalOffset` (`self.TankHull`) (-50.0 0.0 0.0) true false)))

(event `InputAction|Left`
  (params (Key :type "Key Structure")))

(event `InputAction|Right`
  (params (Key :type "Key Structure")))

(fn `UserConstructionScript`)